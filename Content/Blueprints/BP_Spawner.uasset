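; Spawner actor that places BP_FireAi pawns at random points inside one of two box volumes, chosen at random.
; Each spawn line-traces along the pawn's Arrow and takes the hit's Z as its height.
; Tick maps BP_Timer's Seconds to a stepped spawn interval, recreating the looping timer on each change.
; The timer is paused immediately after every creation, and nothing here unpauses it.
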(event `self.ReceiveBeginPlay`
  (bind _returnvalue (`GameplayStatics.GetActorOfClass` "/Game/Blueprints/BP_Timer.BP_Timer_C"))
  (set `self.TimerRef` _returnvalue)
  (`self.CallTimer`))

(event `CallTimer`
  (bind _returnvalue (`KismetSystemLibrary.K2_SetTimerDelegate` (delegate `SpawnerTimer`) (`self.SpawnRate`) true))
  (bind _output_get (set `self.SpawnTimer` _returnvalue))
  (`KismetSystemLibrary.K2_PauseTimerHandle` _output_get))

(event `SpawnerTimer`
  (bind _returnvalue (`self.K2_GetActorLocation` (`self.Actu Ai`)))
  (bind (_returnvalue_x _returnvalue_y) (`KismetMathLibrary.BreakVector` (`self.K2_GetActorLocation` (`self.Actu Ai`))))
  (bind _output_get (set `self.whatbox` (`KismetMathLibrary.RandomInteger` 2)))
  (switch `int` _output_get
    (:`0`
      (bind _actuai (`self.SpawnAi` (`self.Box`)))
      (set `self.Actu Ai` _actuai))
    (:`1`
      (bind _actuai_2 (`self.SpawnAi` (`self.Box2`)))
      (set `self.Actu Ai` _actuai_2)))
  (bind _asbp_fire_ai (cast `/Game/Blueprints/BP_FireAi` (`self.Actu Ai`)))
  (bind _outhit (`KismetSystemLibrary.LineTraceSingle` _returnvalue (+ (* (`SceneComponent.GetForwardVector` (`/Game/Blueprints/BP_FireAi.Arrow` _asbp_fire_ai)) (`self.DistanceRaycast `)) _returnvalue) "TraceTypeQuery1" false (`|MakeArray` (`self.Actu Ai`) self :!type "Actor Object Reference") "None" false))
  (`self.K2_SetActorLocation` (`self.Actu Ai`) (`KismetMathLibrary.MakeVector` _returnvalue_x _returnvalue_y (.z (`.Location` (`GameplayStatics.BreakHitResult` _outhit)))) false false))

(event `self.ReceiveTick`
  (params (DeltaSeconds :type "Float (single-precision)"))
  (bind _returnvalue (select `int` (`self.CheckTime`) :`0` 5.0 :`1` 4.0 :`2` 3.0 :`3` 2.0 :`4` 1.0 :!type "Float (single-precision)"))
  (if (!= _returnvalue (`self.SpawnRate`))
    (set `self.SpawnRate` _returnvalue)
    (`self.CallTimer`)))

(fn `CheckTime`
  (returns (Step :type Integer))
  (bind _timerref (`self.TimerRef`))
  (bind _seconds (`/Game/Blueprints/BP_Timer.Seconds` _timerref))
  (bind _seconds_2 (`/Game/Blueprints/BP_Timer.Seconds` _timerref))
  (return (select `bool` (<= _seconds 30.0) :`false` (select `bool` (<= _seconds_2 60.0) :`false` (select `bool` (<= _seconds_2 90.0) :`false` (select `bool` (<= _seconds 120.0) :`false` (select `bool` (<= (`/Game/Blueprints/BP_Timer.Seconds` _timerref) 150.0) :`true` 1) :`true` 2) :`true` 3) :`true` 4) :`true` 5)))

(fn `SpawnAi`
  (params (Box :type "BoxComponent Object Reference"))
  (returns (ActuAi :type "Pawn Object Reference"))
  (bind (_origin _boxextent) (`KismetSystemLibrary.GetComponentBounds` Box))
  (bind _returnvalue (`AIBlueprintHelperLibrary.SpawnAIFromClass` "/Game/Blueprints/BP_FireAi.BP_FireAi_C" null (`KismetMathLibrary.RandomPointInBoundingBox` _origin _boxextent) (struct) false null))
  (return _returnvalue))

(fn `UserConstructionScript`)