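; BP_PostProcess is an actor that manages saved player settings for screen contrast, gamma and audio volume.
; On BeginPlay it loads or creates a BP_Save, then applies it to the post-process settings and to SFX and Music volumes through a sound mix override.
; It creates the WG_Configue widget with a reference to itself.
; The R key toggles that menu and mouse cursor, saving to the slot on close.
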(event `self.ReceiveBeginPlay`
  (`self.LoadGame`)
  (bind _returnvalue (`|CreateWidget` "/Game/Blueprints/Widgets/WG_Configue.WG_Configue_C" null self))
  (set `self.WidgetRef` _returnvalue)
  (`self.ApplyPostProSettings`)
  (`self.ApplyVolume`))

(event `Key|R`
  (params (Key :type "Key Structure"))
  (bind _widgetref (`self.WidgetRef`))
  (:`Pressed`
    (if (`Widget.IsInViewport` _widgetref)
      (`self.SavePostProSettings`)
      (`Widget.RemoveFromParent` _widgetref)
      (set `PlayerController.bShowMouseCursor` false (`GameplayStatics.GetPlayerController` 0))
      (else
        (`UserWidget.AddToViewport` _widgetref 0)
        (set `PlayerController.bShowMouseCursor` true (`GameplayStatics.GetPlayerController` 0))))))

(fn `ApplyPostProSettings`
  (bind _savegameref (`self.SaveGameRef`))
  (bind _contraste (`/Game/Blueprints/BP_Save.Contraste` _savegameref))
  (bind _luminosity (`/Game/Blueprints/BP_Save.Luminosity` _savegameref))
  (set `PostProcessComponent.Settings` (make `PostProcessSettings` :`ColorContrast` (`KismetMathLibrary.MakeVector4` _contraste _contraste _contraste 1.0) :`ColorGamma` (`KismetMathLibrary.MakeVector4` _luminosity _luminosity _luminosity 1.0)) (`self.PostProcess`)))

(fn `ApplyVolume`
  (bind _savegameref (`self.SaveGameRef`))
  (`GameplayStatics.SetSoundMixClassOverride` "/Game/Audio/MSC_Master.MSC_Master" "/Engine/EngineSounds/SFX.SFX" (`/Game/Blueprints/BP_Save.VolumeFX` _savegameref))
  (`GameplayStatics.SetSoundMixClassOverride` "/Game/Audio/MSC_Master.MSC_Master" "/Engine/EngineSounds/Music.Music" (`/Game/Blueprints/BP_Save.VolumeMusique` _savegameref))
  (`GameplayStatics.PushSoundMixModifier` "/Game/Audio/MSC_Master.MSC_Master"))

(fn `LoadGame`
  ;[0 0 0] Save / Load game
  (bind _returnvalue (`GameplayStatics.DoesSaveGameExist` "Save"))
  (if _returnvalue
    (bind _returnvalue_2 (`GameplayStatics.LoadGameFromSlot` "Save"))
    (bind _asbp_save (cast `/Game/Blueprints/BP_Save` _returnvalue_2))
    (set `self.SaveGameRef` _asbp_save)
    (else
      (bind _returnvalue_3 (`GameplayStatics.CreateSaveGameObject` "/Game/Blueprints/BP_Save.BP_Save_C"))
      (set `self.SaveGameRef` _returnvalue_3))))

(fn `SavePostProSettings`
  (`GameplayStatics.SaveGameToSlot` (`self.SaveGameRef`) "Save"))

(fn `UserConstructionScript`)