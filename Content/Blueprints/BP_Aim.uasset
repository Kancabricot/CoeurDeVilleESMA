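; BP_Aim is an aim actor that supplies an aim direction to the third-person character with the same player index.
; On BeginPlay it searches all BP_ThirdPersonCharacter actors and stores the one whose IndexPlayer matches its own.
; Each tick it sets the Aim component's relative yaw from that player's RotRef, then passes the component's forward vector back through GetGoodForward.
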(event `self.ReceiveBeginPlay`
  (bind _outactors (`GameplayStatics.GetAllActorsOfClass` "/Game/ThirdPerson/Blueprints/BP_ThirdPersonCharacter.BP_ThirdPersonCharacter_C"))
  (for _array_element _outactors
    (bind _asbp_third_person_character (cast `/Game/ThirdPerson/Blueprints/BP_ThirdPersonCharacter` _array_element))
    (if (== (`/Game/ThirdPerson/Blueprints/BP_ThirdPersonCharacter.IndexPlayer` _asbp_third_person_character) (`self.IndexPlayer`))
      (set `self.PlayerRef` _asbp_third_person_character))))

(event `self.ReceiveTick`
  (params (DeltaSeconds :type "Float (single-precision)"))
  (`SceneComponent.K2_SetRelativeRotation` (`self.Aim`) (`KismetMathLibrary.MakeRotator` 0.0 0.0 (`/Game/ThirdPerson/Blueprints/BP_ThirdPersonCharacter.RotRef` (`self.PlayerRef`))) false false)
  (`/Game/ThirdPerson/Blueprints/BP_ThirdPersonCharacter.GetGoodForward` (`self.PlayerRef`) (`SceneComponent.GetForwardVector` (`self.Aim`))))

(fn `UserConstructionScript`)