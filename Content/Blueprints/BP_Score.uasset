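; BP_Score is the score manager that accumulates cleanliness-based points during a run and handles game end.
; On BeginPlay it loads the save through BP_PostProcess, bubble-sorts the parallel score and player arrays ascending, and sends the last entry to the HUD as best score.
; IncrementScore adds the clean percentage while started.
; Enter or Stop clears that flag, shows WG_Score with the score and stops every third-person character.
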(event `self.ReceiveBeginPlay`
  (bind _returnvalue (`GameplayStatics.GetActorOfClass` "/Game/Blueprints/BP_PostProcess.BP_PostProcess_C"))
  (bind _output_get (set `self.SaveRef` _returnvalue))
  (`/Game/Blueprints/BP_PostProcess.LoadGame` _output_get)
  (bind _outactors (`GameplayStatics.GetAllActorsOfClass` "/Game/ThirdPerson/Blueprints/BP_ThirdPersonCharacter.BP_ThirdPersonCharacter_C"))
  (set `self.PlayerRefArray` _outactors)
  (bind _foundwidgets (`WidgetBlueprintLibrary.GetAllWidgetsOfClass` "/Game/Blueprints/Widgets/WG_Hud.WG_Hud_C"))
  (set `self.WGHUDRef` (`|GetArrayItem` _foundwidgets))
  (`self.SortMap`)
  (`self.SetBestScore`))

(event `Key|Enter`
  (params (Key :type "Key Structure"))
  (:`Pressed`
    (set `self.b_IsStarted` false :!label _label)
    (`self.EndGame`)))

(event `/Game/Blueprints/BPI_StartStopGame.Stop`
  (goto _label))

(fn `EndGame`
  (bind _returnvalue (`|CreateWidget` "/Game/Blueprints/Widgets/WG_Score.WG_Score_C" null (`self.Score`)))
  (bind _output_get (set `self.WidgetRef` _returnvalue))
  (`UserWidget.AddToViewport` _output_get 0)
  (for _array_element (`self.PlayerRefArray`)
    (`/Game/ThirdPerson/Blueprints/BP_ThirdPersonCharacter.StopGameEvent` _array_element)))

(fn `IncrementScore`
  (params (PercentDirty :type "Float (double-precision)"))
  (if (`self.b_IsStarted`)
    (set `self.Score` (+ (* (- 1.0 PercentDirty) 100.0) (`self.Score`)))))

(fn `SetBestScore`
  (bind _wghudref (`self.WGHUDRef`))
  (bind _savegameref (`/Game/Blueprints/BP_PostProcess.SaveGameRef` (`self.SaveRef`)))
  (bind _playerarray (`/Game/Blueprints/BP_Save.PlayerArray` _savegameref))
  (bind _scorearray (`/Game/Blueprints/BP_Save.ScoreArray` _savegameref))
  (if (`KismetArrayLibrary.Array_IsEmpty` _scorearray)
    _
    (elif (not (`KismetArrayLibrary.Array_IsEmpty` _playerarray))
      (`/Game/Blueprints/Widgets/WG_Hud.set Score text` _wghudref (`|GetArrayItem` _scorearray (`KismetArrayLibrary.Array_LastIndex` _scorearray)))
      (`/Game/Blueprints/Widgets/WG_Hud.Set Players Names` _wghudref (`|GetArrayItem` _playerarray (`KismetArrayLibrary.Array_LastIndex` _playerarray))))))

(fn `SortMap`
  (locals (LastIndex :type Integer :default 0) (Swapped :type Boolean :default true))
  (bind _savegameref (`/Game/Blueprints/BP_PostProcess.SaveGameRef` (`self.SaveRef`)))
  (bind _scorearray (`/Game/Blueprints/BP_Save.ScoreArray` _savegameref))
  (set `local.LastIndex` (`KismetArrayLibrary.Array_LastIndex` (`/Game/Blueprints/BP_Save.ScoreArray` (`/Game/Blueprints/BP_PostProcess.SaveGameRef` (`self.SaveRef`)))))
  (while (`local.Swapped`)
    (set `local.Swapped` false)
    (for _index (range 1 (+ (`local.LastIndex`) 1))
      (bind _returnvalue (- _index 1))
      (if (> (`|GetArrayItem` _scorearray _returnvalue) (`|GetArrayItem` _scorearray _index))
        (`KismetArrayLibrary.Array_Swap` _scorearray _returnvalue _index)
        (`KismetArrayLibrary.Array_Swap` (`/Game/Blueprints/BP_Save.PlayerArray` _savegameref) _returnvalue _index)
        (set `local.Swapped` true)))))

(fn `UserConstructionScript`)