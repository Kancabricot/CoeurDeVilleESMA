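; BP_Timer is the match countdown that paces dish spawning and signals when time runs out.
; On BeginPlay it caches the dish spawners, players and score actor; Start and Stop toggle the countdown and its music, with Stop playing an end sound.
; Tick advances the Laps struct at fixed time thresholds, triggering spawners whose Order matches the new lap.
; At zero it halts and sends StopMessage to players and score.
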(event `self.ReceiveBeginPlay`
  (set `self.Game Duration (in Seconds)` (`self.Seconds`))
  (bind _outactors (`GameplayStatics.GetAllActorsOfClass` "/Game/Blueprints/BP_DisheSpawner.BP_DisheSpawner_C"))
  (set `self.Dishes` _outactors)
  (bind _outactors_2 (`GameplayStatics.GetAllActorsOfClass` "/Game/ThirdPerson/Blueprints/BP_ThirdPersonCharacter.BP_ThirdPersonCharacter_C"))
  (set `self.PlayerRefArray` _outactors_2)
  (bind _returnvalue (`GameplayStatics.GetActorOfClass` "/Game/Blueprints/BP_Score.BP_Score_C"))
  (set `self.BpScoreRef` _returnvalue))

(event `self.ReceiveTick`
  (params (DeltaSeconds :type "Float (single-precision)"))
  (bind _laps_currentlap (break `/Game/Blueprints/Struct_Laps` (`self.laps`)))
  (if (`self.Can Start Timer`)
    (set `self.Seconds` (- (`self.Seconds`) DeltaSeconds))
    (if (<= (`self.Seconds`) 0.0)
      (set `self.Can Start Timer` false)
      (for _array_element (`self.PlayerRefArray`)
        (message `/Game/Blueprints/BPI_StartStopGame.Stop` _array_element))
      (message `/Game/Blueprints/BPI_StartStopGame.Stop` (`self.BpScoreRef`))
      (else
        (`self.CheckDishesSpawn`)
        (if (`self.CanSpawnDishes`)
          (set `self.CanSpawnDishes` false)
          (for _array_element_2 (`self.Dishes`)
            (if (== _laps_currentlap (`/Game/Blueprints/BP_DisheSpawner.Order` _array_element_2))
              (`/Game/Blueprints/BP_DisheSpawner.Event SpawningDishe` _array_element_2))))))))

(event `/Game/Blueprints/BPI_StartStopGame.Start`
  (set `self.Can Start Timer` true)
  (bind _returnvalue (`GameplayStatics.SpawnSound2D` "/Game/Audio/Ambient/Game_Ost.Game_Ost" 1.0 1.0 0.0 null))
  (set `self.Zouk` _returnvalue))

(event `/Game/Blueprints/BPI_StartStopGame.Stop`
  (set `self.Can Start Timer` false)
  (`AudioComponent.Stop` (`self.Zouk`))
  (`GameplayStatics.SpawnSound2D` "/Game/Audio/Gamestate/Fin_01.Fin_01" 1.0 1.0 0.0 null))

(fn `CheckDishesSpawn`
  (bind _seconds (`self.Seconds`))
  (bind (_laps_currentlap _laps_hasbeenset) (break `/Game/Blueprints/Struct_Laps` (`self.laps`)))
  (bind (_laps_currentlap_2 _laps_hasbeenset_2) (break `/Game/Blueprints/Struct_Laps` (`self.laps`)))
  (bind (_laps_currentlap_3 _laps_hasbeenset_3) (break `/Game/Blueprints/Struct_Laps` (`self.laps`)))
  (bind (_laps_currentlap_4 _laps_hasbeenset_4) (break `/Game/Blueprints/Struct_Laps` (`self.laps`)))
  (if (and (< _seconds 179.0) (not (`|GetArrayItem` _laps_hasbeenset_2)))
    (set `self.laps` (make `/Game/Blueprints/Struct_Laps` 0 (`|MakeArray` true false false false)))
    (set `self.CanSpawnDishes` true :!label _label)
    (elif (and (< _seconds 150.0) (not (`|GetArrayItem` _laps_hasbeenset_3 1)))
      (set `self.laps` (make `/Game/Blueprints/Struct_Laps` 1 (`|MakeArray` true true false false)))
      (goto _label)
      (elif (and (< _seconds 120.0) (not (`|GetArrayItem` _laps_hasbeenset_4 2)))
        (set `self.laps` (make `/Game/Blueprints/Struct_Laps` 2 (`|MakeArray` true true true false)))
        (goto _label)
        (elif (and (< _seconds 90.0) (not (`|GetArrayItem` _laps_hasbeenset 3)))
          (set `self.laps` (make `/Game/Blueprints/Struct_Laps` 3 (`|MakeArray` true true true true)))
          (goto _label)
          (else
            _)))))
  (return))

(fn `UserConstructionScript`)