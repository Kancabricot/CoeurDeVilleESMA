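; Fire enemy AI that scales up on spawn, wanders to random navmesh points, and after a delay grows larger and explodes, spawning an explosion brush.
; GetHit shrinks its mesh and RVT brush; below a threshold it dies with VFX, sound, score popup and points.
; Capsule overlap pushes the player along their arrow's direction, with a cooldown.
; The looping timer's event is empty and visibility-toggle logic is disconnected.
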(event `self.Capsule.OnComponentBeginOverlap`
  (params (OverlappedComponent :type "PrimitiveComponent Object Reference") (OtherActor :type "Actor Object Reference") (OtherComp :type "PrimitiveComponent Object Reference") (OtherBodyIndex :type Integer) (bFromSweep :type Boolean) (SweepResult :type "HitResult Structure (by ref)"))
  (bind _asbp_third_person_character (cast `/Game/ThirdPerson/Blueprints/BP_ThirdPersonCharacter` OtherActor))
  (set `self.ActuPlayerHit` _asbp_third_person_character)
  (if (`self.CanPush`)
    (set `MovementComponent.Velocity` (* (`SceneComponent.GetForwardVector` (`/Game/ThirdPerson/Blueprints/BP_ThirdPersonCharacter.Arrow1` _asbp_third_person_character)) 100.0) (`Character.CharacterMovement` _asbp_third_person_character))
    (set `self.CanPush` false)
    (bind _returnvalue (`KismetSystemLibrary.K2_SetTimerDelegate` (delegate `Event`) 0.3 true))
    (set `self.Timer` _returnvalue)
    (`KismetSystemLibrary.Delay` (`self.Invisibilty`))
    (set `self.CanPush` true)
    (`KismetSystemLibrary.K2_PauseTimerHandle` (`self.Timer`))))

(event `Event`)

(event `self.ReceiveBeginPlay`
  (`|ExecutionSequence`
    (:`then_0`
      (bind _returnvalue (`GameplayStatics.GetActorOfClass` "/Game/Blueprints/BP_Spawner.BP_Spawner_C"))
      (set `self.Spawner` _returnvalue))
    (:`then_1`
      (bind (_direction _newtrack_0) (`Timeline|Scale`)
        (:`Update`
          (bind _returnvalue_2 (`KismetMathLibrary.Lerp` 0.0 0.5 _newtrack_0))
          (`self.SetActorScale3D` (`KismetMathLibrary.MakeVector` _returnvalue_2 _returnvalue_2 _returnvalue_2)))))
    (:`then_2`
      (`KismetSystemLibrary.Delay` 0.2)
      (`self.WanderAround`))
    (:`then_3`
      (`KismetSystemLibrary.Delay` 12.0)
      (bind (_direction_2 _newtrack_0_2) (`Timeline|Timeline` :!via `PlayFromStart`)
        (:`Update`
          (bind _returnvalue_3 (`KismetMathLibrary.Lerp` 0.5 1.0 _newtrack_0_2))
          (`self.SetActorScale3D` (`KismetMathLibrary.MakeVector` _returnvalue_3 _returnvalue_3 _returnvalue_3)))
        (:`Finished`
          (`self.Explosion`))))))

(event `Wander`
  (bind _randomlocation (`NavigationSystemV1.K2_GetRandomLocationInNavigableRadius` (`self.K2_GetActorLocation`) 100000.0 null null :!label _label))
  (`AITask_MoveTo.AIMoveTo` (`AIBlueprintHelperLibrary.GetAIController` (`self.GetController`)) _randomlocation null
    (:`OnMoveFinished`
      (`KismetSystemLibrary.Delay` 1.0)
      (goto _label))))

(event `/Game/Blueprints/BPI_Hit.GetHit`
  (bind _planebrushrvt (`self.PlaneBrushRVT`))
  (bind _spawnmanagerref (`self.SpawnManagerRef`))
  (bind _v2 (`self.v2`))
  (bind _returnvalue_x (`KismetMathLibrary.BreakVector` (`SceneComponent.K2_GetComponentScale` _v2)))
  (bind _screenposition (`WidgetLayoutLibrary.ProjectWorldLocationToWidgetPosition` (`GameplayStatics.GetPlayerController` 0) (`SceneComponent.K2_GetComponentLocation` (`self.Niagara`)) true))
  (`SceneComponent.SetWorldScale3D` _v2 (- (`SceneComponent.K2_GetComponentScale` _v2) 0.1))
  (`SceneComponent.SetWorldScale3D` _planebrushrvt (- (`SceneComponent.K2_GetComponentScale` _planebrushrvt) 0.01))
  (if (<= _returnvalue_x 1.0)
    (`GameplayStatics.SpawnSound2D` "/Game/Audio/Mob/SC_Mort_mob.SC_Mort_mob" 2.0 1.0 0.0 null)
    (`NiagaraFunctionLibrary.SpawnSystemAtLocation` "/Game/VFX/Death_POOF/ns_DeathVFX.ns_DeathVFX" (`self.K2_GetActorLocation`))
    (bind _returnvalue (`|CreateWidget` "/Game/Blueprints/Widgets/WG_ScorePopUp.WG_ScorePopUp_C"))
    (`UserWidget.SetPositionInViewport` _returnvalue (`KismetMathLibrary.MakeVector2D` (`KismetMathLibrary.BreakVector2D` _screenposition) (+ (`.Y` (`KismetMathLibrary.BreakVector2D` _screenposition)) -100.0)) true)
    (`/Game/Blueprints/Widgets/WG_ScorePopUp.Spawn WinScore` _returnvalue 100)
    (set `/Game/Blueprints/BP_SpawnManager.Score` (+ (`/Game/Blueprints/BP_SpawnManager.Score` _spawnmanagerref) 100) _spawnmanagerref)
    (`UserWidget.AddToViewport` _returnvalue 0)
    (`self.K2_DestroyActor`)))

(fn `Explosion`
  (bind (_returnvalue_location _returnvalue_rotation) (`KismetMathLibrary.BreakTransform` (`SceneComponent.K2_GetComponentToWorld` (`self.v2`))))
  (`|SpawnActorFromClass` "/Game/Blueprints/BP_ExplosionBrush.BP_ExplosionBrush_C" (`KismetMathLibrary.MakeTransform` _returnvalue_location _returnvalue_rotation) "Undefined" "MultiplyWithRoot" null "/Game/TestRVT/M_BrushExplosion.M_BrushExplosion" null)
  (`GameplayStatics.SpawnSound2D` "/Game/Audio/Mob/Splurt_02.Splurt_02" 1.0 1.0 0.0 null)
  (`self.K2_DestroyActor`))

(fn `UserConstructionScript`)

(fn `WanderAround`
  (`self.Wander`))