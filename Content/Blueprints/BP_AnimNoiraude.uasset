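; BP_AnimNoiraude is an actor that drifts along the Y axis once play begins, then destroys itself.
; A slowed Timeline drives a Lerp from the current Y to a small offset, so movement accumulates each update rather than following fixed endpoints.
; The construction script prints a debug "Hello" for each component overlapping its Box, whose begin-overlap event is empty.
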(event `self.ReceiveBeginPlay`
  (bind (_returnvalue_x _returnvalue_y _returnvalue_z) (`KismetMathLibrary.BreakVector` (`self.K2_GetActorLocation`)))
  (`TimelineComponent.SetPlayRate` (`self.Timeline`) 0.4)
  (bind (_direction _newtrack_0) (`Timeline|Timeline` :!via `PlayFromStart`)
    (:`Update`
      (`self.K2_SetActorLocation` (`KismetMathLibrary.MakeVector` _returnvalue_x (`KismetMathLibrary.Lerp` _returnvalue_y (+ _returnvalue_y 2.0) _newtrack_0) _returnvalue_z)))
    (:`Finished`
      (`self.K2_DestroyActor`))))

(event `self.Box.OnComponentBeginOverlap`
  (params (OverlappedComponent :type "PrimitiveComponent Object Reference") (OtherActor :type "Actor Object Reference") (OtherComp :type "PrimitiveComponent Object Reference") (OtherBodyIndex :type Integer) (bFromSweep :type Boolean) (SweepResult :type "HitResult Structure (by ref)")))

(fn `UserConstructionScript`
  (bind _box (`self.Box`))
  (bind _outcomponents (`KismetSystemLibrary.ComponentOverlapComponents` _box (`SceneComponent.K2_GetComponentToWorld` _box) (`|MakeArray` "ObjectTypeQuery1" "ObjectTypeQuery2" "ObjectTypeQuery3" "ObjectTypeQuery4" :!type "EObjectTypeQuery Enum")))
  (for _array_element _outcomponents
    (`KismetSystemLibrary.PrintString` "Hello")))