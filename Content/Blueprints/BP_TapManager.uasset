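; BP_TapManager manages the filling of all Bp_WaterWindow actors in the level.
; On BeginPlay it gathers them, shuffles them, fills the first two, and starts checking once a timeline finishes.
; Each check shuffles the list and fills the first window at or below half on FillEmpty.
; Checks repeat through a delay-driven wait loop, with a timeline after each fill also leading back into the wait.
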(event `self.ReceiveBeginPlay`
  (bind _outactors (`GameplayStatics.GetAllActorsOfClass` "/Game/ThirdPerson/Blueprints/Bp_WaterWindow.Bp_WaterWindow_C"))
  (set `self.WaterWindows Refs` _outactors)
  (`self.Fill the two first windows`))

(event `Fill the two first windows`
  (bind _waterwindows_refs (`self.WaterWindows Refs`))
  ;[1 1 1] Fill the two first Windows
  (`KismetArrayLibrary.Array_Shuffle` _waterwindows_refs)
  (`/Game/ThirdPerson/Blueprints/Bp_WaterWindow.FillWater` (`|GetArrayItem` _waterwindows_refs))
  (`/Game/ThirdPerson/Blueprints/Bp_WaterWindow.FillWater` (`|GetArrayItem` _waterwindows_refs 1))
  (`Timeline|Timeline` :!via `PlayFromStart`
    (:`Finished`
      (`self.Check Water Windows`))))

(event `Wait`
  ;[0.1719 0.1719 0.1719] Wait
  (`KismetSystemLibrary.Delay` (`self.Wait Duration`))
  (`self.Check Water Windows`))

(event `Check Water Windows`
  (bind _waterwindows_refs (`self.WaterWindows Refs`))
  ;[0.1719 0.1719 0.1719] Check if Water Window is empty
  (`KismetArrayLibrary.Array_Shuffle` _waterwindows_refs)
  (for _array_element _waterwindows_refs
    (set `self.Water Window Ref` _array_element)
    (if (<= (`/Game/ThirdPerson/Blueprints/Bp_WaterWindow.Fill Empty` (`self.Water Window Ref`)) 0.5)
      (`self.Fill Water Windows`)
      (break)))
  (`self.Wait`))

(event `Fill Water Windows`
  ;[0.1719 0.1719 0.1719] Fill Water Windows
  (`/Game/ThirdPerson/Blueprints/Bp_WaterWindow.FillWater` (`self.Water Window Ref`))
  (`Timeline|TL_FillWaterWindows` :!via `PlayFromStart`
    (:`Finished`
      (`self.Wait`))))

(fn `UserConstructionScript`)