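; BP_SpawnManager runs a timed local-multiplayer round, from tutorial to score screen.
; On BeginPlay it possesses a character per PlayerStart, links the spawner and HUD, loads post-process settings and starts menu music.
; A looping timer polls the Runtime Virtual Texture volume's dirty percentage, spawning a tutorial AI once nearly clean.
; Start triggers the spawner, game music and Tick countdown; at zero it stops players, shows the score and plays end audio.
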(event `self.ReceiveBeginPlay`
  (`self.CreatePlayers`)
  (set `self.Game Duration (in Seconds)` (`self.Seconds`))
  (bind _returnvalue (`GameplayStatics.GetActorOfClass` "/Game/Blueprints/BP_Spawner.BP_Spawner_C"))
  (bind _output_get (set `self.SpawnerRef` _returnvalue))
  (`/Game/Blueprints/BP_Spawner.GetSpawnManagerRef` _output_get self)
  (bind _returnvalue_2 (`GameplayStatics.GetActorOfClass` "/Game/Blueprints/BP_PostProcess.BP_PostProcess_C"))
  (bind _output_get_2 (set `self.SavePostProRef` _returnvalue_2))
  (`/Game/Blueprints/BP_PostProcess.LoadGame` _output_get_2)
  (bind _returnvalue_3 (`|CreateWidget` "/Game/Blueprints/Widgets/WG_Hud.WG_Hud_C" null self))
  (bind _output_get_3 (set `self.WGHudRef` _returnvalue_3))
  (`UserWidget.AddToViewport` _output_get_3 0)
  (bind _returnvalue_4 (`GameplayStatics.GetActorOfClass` "/Game/Blueprints/Runtime_Virtual_Texture_Volume_Blueprint.Runtime_Virtual_Texture_Volume_Blueprint_C"))
  (set `self.RVTRef` _returnvalue_4)
  (bind _returnvalue_5 (`GameplayStatics.SpawnSound2D` "/Game/Audio/Ambient/Menu_01.Menu_01" 1.0 1.0 0.0 null))
  (set `self.Zouk` _returnvalue_5)
  (bind _returnvalue_6 (`KismetSystemLibrary.K2_SetTimerDelegate` (delegate `CheckDirtyTuto`) 0.5 true))
  (set `self.TimerEventRef` _returnvalue_6))

(event `CheckDirtyTuto`
  (if (< (`/Game/Blueprints/Runtime_Virtual_Texture_Volume_Blueprint.GetPercentDirty` (`self.RVTRef`)) 0.015)
    (`KismetSystemLibrary.K2_PauseTimerHandle` (`self.TimerEventRef`))
    (`|SpawnActorFromClass` "/Game/Blueprints/BP_AITuto.BP_AITuto_C" (`KismetMathLibrary.MakeTransform` (0.0 0.0 0.0)) "Undefined" "MultiplyWithRoot" null null null)
    (`/Game/Blueprints/Widgets/WG_Hud.TextTuto` (`self.WGHudRef`))))

(event `self.ReceiveTick`
  (params (DeltaSeconds :type "Float (single-precision)"))
  (if (`self.Can Start Timer`)
    (set `self.Seconds` (- (`self.Seconds`) DeltaSeconds))
    (if (<= (`self.Seconds`) 0.0)
      (set `self.Can Start Timer` false)
      (for _array_element (`self.PlayerRefArray`)
        (message `/Game/Blueprints/BPI_StartStopGame.Stop` _array_element))
      (`self.EndGame`)
      (`AudioComponent.Stop` (`self.Zouk`))
      (`GameplayStatics.SpawnSound2D` "/Game/Audio/Gamestate/Fin_01.Fin_01" 1.0 1.0 0.0 null))))

(fn `CreatePlayers`
  (bind _outactors (`GameplayStatics.GetAllActorsOfClass` "/Script/Engine.PlayerStart"))
  (for (_array_element _array_index) _outactors
    (`GameplayStatics.CreatePlayer` _array_index)
    (bind _returnvalue (`|SpawnActorFromClass` "/Game/ThirdPerson/Blueprints/BP_ThirdPersonCharacter.BP_ThirdPersonCharacter_C" (`self.GetTransform` _array_element) "Undefined" "MultiplyWithRoot" null _array_index self null))
    (`Controller.Possess` (`GameplayStatics.GetPlayerController` _array_index) _returnvalue)
    (`KismetArrayLibrary.Array_Add` (`self.PlayerRefArray`) _returnvalue)))

(fn `EndGame`
  (bind _returnvalue (`|CreateWidget` "/Game/Blueprints/Widgets/WG_Score.WG_Score_C" null (`self.Score`)))
  (bind _output_get (set `self.WGScoreRef` _returnvalue))
  (`UserWidget.AddToViewport` _output_get 0)
  (for _array_element (`self.PlayerRefArray`)
    (`/Game/ThirdPerson/Blueprints/BP_ThirdPersonCharacter.StopGameEvent` _array_element)))

(fn `Start`
  (bind _spawnerref (`self.SpawnerRef`))
  (set `self.Can Start Timer` true)
  (`/Engine/EditorBlueprintResources/StandardMacros.IsValid` _spawnerref
    (:`Is Valid`
      (`/Game/Blueprints/BP_Spawner.CallTimer` _spawnerref)
      (`/Game/Blueprints/Widgets/WG_Hud.DeleteWid` (`self.WGHudRef`))
      (bind _returnvalue (`GameplayStatics.SpawnSound2D` "/Game/Audio/Ambient/Game_Ost.Game_Ost" 1.0 1.0 0.0 null))
      (set `self.Zouk` _returnvalue))))

(fn `UserConstructionScript`)