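; Tutorial AI mob (per its name) that wanders the navmesh and spawns a brush explosion after 15 seconds, destroying itself.
; Touching a player launches them along their arrow and blinks their mesh during a push cooldown.
; ChooseWhatDish, not called here, targets a random not-fully-dirty dish, which the mob dirties on overlap before dying.
; GetHit shrinks the mob and its RVT brush plane until it dies.
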(event `self.Capsule.OnComponentBeginOverlap`
  (params (OverlappedComponent :type "PrimitiveComponent Object Reference") (OtherActor :type "Actor Object Reference") (OtherComp :type "PrimitiveComponent Object Reference") (OtherBodyIndex :type Integer) (bFromSweep :type Boolean) (SweepResult :type "HitResult Structure (by ref)"))
  (if (== OtherActor (`self.target`))
    (`/Game/Blueprints/BP_Dishe.DirtPlate` (`self.target`))
    (`GameplayStatics.SpawnSound2D` "/Game/Audio/Mob/Splurt_02.Splurt_02" 1.0 1.0 0.0 null)
    (`self.K2_DestroyActor`)
    (else
      (bind _asbp_third_person_character (cast `/Game/ThirdPerson/Blueprints/BP_ThirdPersonCharacter` OtherActor))
      (set `self.ActuPlayerHit` _asbp_third_person_character)
      (if (`self.CanPush`)
        (set `MovementComponent.Velocity` (* (`SceneComponent.GetForwardVector` (`/Game/ThirdPerson/Blueprints/BP_ThirdPersonCharacter.Arrow1` _asbp_third_person_character)) 10000.0) (`Character.CharacterMovement` _asbp_third_person_character))
        (set `self.CanPush` false)
        (bind _returnvalue (`KismetSystemLibrary.K2_SetTimerDelegate` (delegate `Event`) 0.3 true))
        (set `self.Timer` _returnvalue)
        (`KismetSystemLibrary.Delay` (`self.Invisibilty`))
        (set `self.CanPush` true)
        (`KismetSystemLibrary.K2_PauseTimerHandle` (`self.Timer`))
        (`SceneComponent.SetVisibility` (`/Game/ThirdPerson/Blueprints/BP_ThirdPersonCharacter.StaticMesh` (`self.ActuPlayerHit`)) true false)))))

(event `Event`
  (bind _staticmesh (`/Game/ThirdPerson/Blueprints/BP_ThirdPersonCharacter.StaticMesh` (`self.ActuPlayerHit`)))
  (`/Engine/EditorBlueprintResources/StandardMacros.FlipFlop`
    (:`A`
      (`SceneComponent.SetVisibility` _staticmesh false false))
    (:`B`
      (`SceneComponent.SetVisibility` _staticmesh true false))))

(event `self.ReceiveBeginPlay`
  (`|ExecutionSequence`
    (:`then_0`
      (bind _outactors (`GameplayStatics.GetAllActorsOfClass` "/Game/Blueprints/BP_Dishe.BP_Dishe_C"))
      (set `self.AllDishs` _outactors)
      (bind _returnvalue (`GameplayStatics.GetActorOfClass` "/Game/Blueprints/BP_Spawner.BP_Spawner_C"))
      (set `self.Spawner` _returnvalue))
    (:`then_1`
      (`KismetSystemLibrary.Delay` 0.2)
      (`self.WanderAround`))
    (:`then_2`
      (`KismetSystemLibrary.Delay` 15.0)
      (`self.Explosion`))))

(event `Wander`
  (bind _randomlocation (`NavigationSystemV1.K2_GetRandomLocationInNavigableRadius` (`self.K2_GetActorLocation`) 100000.0 null null :!label _label))
  (`AITask_MoveTo.AIMoveTo` (`AIBlueprintHelperLibrary.GetAIController` (`self.GetController`)) _randomlocation null
    (:`OnMoveFinished`
      (`KismetSystemLibrary.Delay` 1.0)
      (goto _label))))

(event `ChooseWhatDish`
  (`KismetArrayLibrary.Array_Shuffle` (`self.AllDishs`))
  (for _array_element (`self.AllDishs`)
    (if (not (>= (`/Game/Blueprints/BP_Dishe.Dirt` _array_element) 1.0))
      (bind _output_get (set `self.target` _array_element))
      (`KismetArrayLibrary.Array_Add` (`/Game/Blueprints/BP_Dishe.whosIsYourtarget` _output_get) self)
      (break)))
  (if (== (`self.target`) null)
    (`self.WanderAround`)
    (bind (_direction _newtrack_0) (`Timeline|TimelineAnim` :!label _label_2)
      (:`Update`
        (`SceneComponent.SetRelativeScale3D` (`self.Niagara`) (`KismetMathLibrary.MakeVector` _newtrack_0 _newtrack_0 1.0))))
    (else
      (`AIController.MoveToActor` (`AIBlueprintHelperLibrary.GetAIController` (`self.GetController`)) (`self.target`) -1.0 false true true null true)
      (goto _label_2))))

(event `/Game/Blueprints/BPI_Hit.GetHit`
  (bind _planebrushrvt (`self.PlaneBrushRVT`))
  (bind _v2 (`self.v2`))
  (bind _returnvalue_x (`KismetMathLibrary.BreakVector` (`SceneComponent.K2_GetComponentScale` _v2)))
  (`SceneComponent.SetWorldScale3D` _v2 (- (`SceneComponent.K2_GetComponentScale` _v2) 0.1))
  (`SceneComponent.SetWorldScale3D` _planebrushrvt (- (`SceneComponent.K2_GetComponentScale` _planebrushrvt) 0.01))
  (if (<= _returnvalue_x 1.0)
    (`GameplayStatics.SpawnSound2D` "/Game/Audio/Mob/SC_Mort_mob.SC_Mort_mob" 2.0 1.0 0.0 null)
    (`self.K2_DestroyActor`)))

(fn `Explosion`
  (`|SpawnActorFromClass` "/Game/Blueprints/BP_ExplosionBrush.BP_ExplosionBrush_C" (`SceneComponent.K2_GetComponentToWorld` (`self.v2`)) "Undefined" "MultiplyWithRoot" null "/Game/TestRVT/M_BrushExplosion.M_BrushExplosion" null)
  (`self.K2_DestroyActor`))

(fn `UserConstructionScript`)

(fn `WanderAround`
  (`self.Wander`))