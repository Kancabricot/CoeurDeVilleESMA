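; BP_Dishe is a dish that fire AI dirty and water projectiles clean through its clamped Dirt value.
; While mostly clean, it adds a point to BP_Score every second.
; A hit leaving it fully dirty increments the spawner's dish count and makes the AI in its target list choose again.
; When that count hits fifteen, it instead pauses spawning and sets every fire AI on a looping wander timer.
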(event `self.ReceiveTick`
  (params (DeltaSeconds :type "Float (single-precision)"))
  ;[1 1 1] 1
)

(event `self.ReceiveBeginPlay`
  (`|ExecutionSequence`
    (:`then_0`
      (bind _returnvalue (`GameplayStatics.GetActorOfClass` "/Game/Blueprints/BP_Spawner.BP_Spawner_C"))
      (set `self.SpawnerAiRef` _returnvalue))
    (:`then_1`
      (bind _returnvalue_2 (`GameplayStatics.GetActorOfClass` "/Game/Blueprints/BP_Score.BP_Score_C"))
      (`KismetSystemLibrary.Delay` 1.0 :!label _label)
      (if (<= (`self.Dirt`) 0.35)
        (set `/Game/Blueprints/BP_Score.Score` (+ (`/Game/Blueprints/BP_Score.Score` _returnvalue_2) 1) _returnvalue_2)
        (goto _label)
        (else
          (goto _label))))))

(event `DirtPlate`
  (params (Overlapper :type "Actor Object Reference"))
  (cast `/Game/Blueprints/BP_FireAi` Overlapper
    (:`then`
      (`self.SetDirt` 0.3))
    (:`CastFailed`
      (cast `/Game/ThirdPerson/Blueprints/BP_PojectilWater` Overlapper)
      (`self.SetDirt` -0.01))))

(fn `SetDirt`
  (params (`Dirt Transform` :type "Float (double-precision)"))
  (bind _spawnerairef (`self.SpawnerAiRef`))
  (bind _output_get (set `self.Dirt` (`KismetMathLibrary.FClamp` (+ `Dirt Transform` (`self.Dirt`)) 0.1)))
  (if (== (`KismetMathLibrary.SelectFloat` 0.0 _output_get (<= _output_get 0.35)) 1.0)
    (`/Engine/EditorBlueprintResources/StandardMacros.IncrementInt` (`/Game/Blueprints/BP_Spawner.NbDish` _spawnerairef)
      (:`  `
        (if (== (`/Game/Blueprints/BP_Spawner.NbDish` _spawnerairef) 15)
          (`KismetSystemLibrary.K2_PauseTimerHandle` (`/Game/Blueprints/BP_Spawner.SpawnTimer` (`self.SpawnerAiRef`)))
          (bind _outactors (`GameplayStatics.GetAllActorsOfClass` "/Game/Blueprints/BP_FireAi.BP_FireAi_C"))
          (for _array_element _outactors
            (`KismetSystemLibrary.K2_SetTimer` _array_element "WanderAround" 5.0 true -5.0)
            (`KismetSystemLibrary.PrintString` "WANDER"))
          (else
            (for _array_element_2 (`self.whosIsYourtarget`)
              (`/Game/Blueprints/BP_FireAi.ChooseWhatDish` _array_element_2))
            (return)))))
    (else
      (return))))

(fn `UserConstructionScript`)