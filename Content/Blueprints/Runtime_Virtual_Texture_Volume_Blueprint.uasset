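; Runtime Virtual Texture volume Blueprint that tracks how dirty a surface is and feeds that into the HUD score.
; Clears two render targets at start, then draws M_DrawToRT into both every tick.
; Once started with a spawn manager reference, a one-second looping timer reads back the score target and passes the fraction of pixels with non-zero red to IncrementScore.
; The readback also prints debug totals.
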(event `self.ReceiveBeginPlay`
  (`KismetRenderingLibrary.ClearRenderTarget2D` "/Game/TestRVT/RT_ScoreTarget.RT_ScoreTarget")
  (`KismetRenderingLibrary.ClearRenderTarget2D` "/Game/TestRVT/RT_Catcher.RT_Catcher"))

(event `StartIcrementation`
  (params (SpawnManagerRef :type "/Game/Blueprints/BP_SpawnManager Object Reference"))
  (set `self.SpawnManagerRef` SpawnManagerRef)
  (`KismetSystemLibrary.K2_SetTimerDelegate` (delegate `SamplePixels`) 1.0 true -1.0))

(event `SamplePixels`
  (`/Game/Blueprints/Widgets/WG_Hud.IncrementScore` (`/Game/Blueprints/BP_SpawnManager.WGHudRef` (`self.SpawnManagerRef`)) (`self.GetPercentDirty`)))

(event `self.ReceiveTick`
  (params (DeltaSeconds :type "Float (single-precision)"))
  (`KismetRenderingLibrary.DrawMaterialToRenderTarget` "/Game/TestRVT/RT_Catcher.RT_Catcher" "/Game/TestRVT/M_DrawToRT.M_DrawToRT")
  (`KismetRenderingLibrary.DrawMaterialToRenderTarget` "/Game/TestRVT/RT_ScoreTarget.RT_ScoreTarget" "/Game/TestRVT/M_DrawToRT.M_DrawToRT"))

(fn `GetPercentDirty`
  (returns (PercentDirty :type "Float (double-precision)"))
  (locals (Sum :type Integer) (nbPixels :type Integer :default 0) (PixelsInfos :type "Array of Color Structure"))
  (bind _returnvalue (/ (`KismetMathLibrary.Conv_IntToDouble` (`local.Sum`)) (`KismetMathLibrary.Conv_IntToDouble` (`local.nbPixels`))))
  (bind _outsamples (`KismetRenderingLibrary.ReadRenderTarget` "/Game/TestRVT/RT_ScoreTarget.RT_ScoreTarget"))
  (set `local.PixelsInfos` _outsamples)
  (set `local.nbPixels` (`KismetArrayLibrary.Array_Length` _outsamples))
  (for _array_element (`local.PixelsInfos`)
    (set `local.Sum` (+ (`local.Sum`) (select `bool` (> (`.R` (break `Color` _array_element)) 0) :`true` 1))))
  (`KismetSystemLibrary.PrintString` (`KismetStringLibrary.Concat_StrStr` "Pixels : " (`KismetStringLibrary.Conv_IntToString` (`local.nbPixels`)) "  Sum : " (`KismetStringLibrary.Conv_IntToString` (`local.Sum`)) "  Avg : " (`KismetStringLibrary.Conv_DoubleToString` _returnvalue)))
  (return _returnvalue))

(fn `UserConstructionScript`)