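; BP_AITuto is a tutorial AI mob that patrols back and forth along the spline of a BP_SplineTuto actor.
; A slowed timeline lerps distance along the spline to set its transform, and a FlipFlop on finish alternates reverse and forward runs.
; Each GetHit shrinks its mesh and RVT brush; at minimum scale it plays death sound and VFX, calls Start on BP_SpawnManager, then destroys itself.
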(event `self.ReceiveBeginPlay`
  (`|ExecutionSequence`
    (:`then_0`
      (bind _returnvalue (`GameplayStatics.GetActorOfClass` "/Game/Blueprints/BP_SplineTuto.BP_SplineTuto_C"))
      (set `self.SplineRef` _returnvalue)
      (`TimelineComponent.SetPlayRate` (`self.Timeline`) 0.2)
      (bind _returnvalue_2 (`GameplayStatics.GetActorOfClass` "/Game/Blueprints/BP_SpawnManager.BP_SpawnManager_C"))
      (set `self.SpawnManagerRef` _returnvalue_2))
    (:`then_1`
      (`self.Play`))))

(event `Play`
  (bind _spline (`/Game/Blueprints/BP_SplineTuto.Spline` (`self.SplineRef`)))
  (bind (_direction _movement_track) (`Timeline|Timeline` :!via `PlayFromStart` :!label _label)
    (:`Update`
      (bind _returnvalue (`KismetMathLibrary.Lerp` 0.0 (`SplineComponent.GetSplineLength` (`/Game/Blueprints/BP_SplineTuto.Spline` (`self.SplineRef`))) _movement_track))
      (`self.K2_SetActorTransform` (`KismetMathLibrary.MakeTransform` (`SplineComponent.GetLocationAtDistanceAlongSpline` _spline _returnvalue "World") (`SplineComponent.GetRotationAtDistanceAlongSpline` _spline _returnvalue "Local"))))
    (:`Finished`
      (`/Engine/EditorBlueprintResources/StandardMacros.FlipFlop`
        (:`A`
          (`self.Reverse`))
        (:`B`
          (`self.Play`))))))

(event `Reverse`
  (goto _label :!via `ReverseFromEnd`))

(event `/Game/Blueprints/BPI_Hit.GetHit`
  (params (PlayerRef :type "/Game/ThirdPerson/Blueprints/BP_ThirdPersonCharacter Object Reference"))
  (bind _planebrushrvt (`self.PlaneBrushRVT`))
  (bind _v2 (`self.v2`))
  (bind _returnvalue_x (`KismetMathLibrary.BreakVector` (`SceneComponent.K2_GetComponentScale` _v2)))
  (`SceneComponent.SetWorldScale3D` _v2 (- (`SceneComponent.K2_GetComponentScale` _v2) 0.1))
  (`SceneComponent.SetWorldScale3D` _planebrushrvt (- (`SceneComponent.K2_GetComponentScale` _planebrushrvt) 0.01))
  (if (<= _returnvalue_x 1.0)
    (`GameplayStatics.SpawnSound2D` "/Game/Audio/Mob/SC_Mort_mob.SC_Mort_mob" 2.0 1.0 0.0 null)
    (`NiagaraFunctionLibrary.SpawnSystemAtLocation` "/Game/VFX/Death_POOF/ns_DeathVFX.ns_DeathVFX" (`self.K2_GetActorLocation`))
    (`self.Die`)))

(fn `Die`
  (`/Game/Blueprints/BP_SpawnManager.Start` (`self.SpawnManagerRef`))
  (`self.K2_DestroyActor`))

(fn `UserConstructionScript`)