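; Tutorial dish actor that the player cleans by hitting it, with a widget bar showing its remaining dirtiness.
; Each hit lowers Dirtiness by a fixed step, refreshes the bar and applies a sand material, flagging the dish clean once no further step fits.
; When the first two tutorial dishes found in the level are both clean, it tells BP_Tuto to start the game.
; A Start event destroys the dish.
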(event `self.ReceiveBeginPlay`
  (`self.set Dirtiness Bar`)
  (bind _outactors (`GameplayStatics.GetAllActorsOfClass` "BP_Tuto_Dishe_C"))
  (set `self.Tuto Dishes Ref` _outactors)
  (bind _returnvalue (`GameplayStatics.GetActorOfClass` "/Game/Blueprints/Tuto/BP_Tuto.BP_Tuto_C"))
  (set `self.tutoRef` _returnvalue))

(event `Event Clean Dishe`
  (bind _tuto_dishes_ref (`self.Tuto Dishes Ref`))
  (`self.cleanDishe`)
  (`PrimitiveComponent.SetMaterial` (`self.StaticMesh`) 0 "/Game/Enviro/Material/M_Sand1.M_Sand1")
  (if (and (`/Game/Blueprints/Tuto/BP_Tuto_Dishe.IsClean` (`|GetArrayItem` _tuto_dishes_ref)) (`/Game/Blueprints/Tuto/BP_Tuto_Dishe.IsClean` (`|GetArrayItem` _tuto_dishes_ref 1)))
    (`/Game/Blueprints/Tuto/BP_Tuto.Start Game` (`self.tutoRef`))))

(event `/Game/Blueprints/BPI_StartStopGame.Start`
  (`self.K2_DestroyActor`))

(event `/Game/Blueprints/BPI_Hit.GetHit`
  (`self.Event Clean Dishe`))

(fn `cleanDishe`
  (bind _returnvalue (+ (`self.Dirtiness`) -0.1))
  (if (>= _returnvalue 0.0)
    (set `self.Dirtiness` _returnvalue)
    (`self.set Dirtiness Bar`)
    (else
      (set `self.IsClean` true)
      (return))))

(fn `set Dirtiness Bar`
  (bind _aswg_dirtiness (cast `/Game/Blueprints/Widgets/WG_Dirtiness` (`WidgetComponent.GetUserWidgetObject` (`self.Widget`))))
  (set `/Game/Blueprints/Widgets/WG_Dirtiness.Dirtiness` (`self.Dirtiness`) _aswg_dirtiness))

(fn `UserConstructionScript`)