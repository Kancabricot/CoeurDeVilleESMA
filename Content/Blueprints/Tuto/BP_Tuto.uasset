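; BP_Tuto is a tutorial controller that holds the tutorial dishes and HUD and tears them down when the game starts.
; BeginPlay gathers every BP_Tuto_Dishe, grabs the first top-level WG_Hud widget and plays the Menu_01 sound in 2D.
; The StartGame event destroys each gathered dish and calls DeleteWid on the HUD, leaving the spawned music reference untouched.
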(event `self.ReceiveBeginPlay`
  (bind _outactors (`GameplayStatics.GetAllActorsOfClass` "/Game/Blueprints/Tuto/BP_Tuto_Dishe.BP_Tuto_Dishe_C"))
  (set `self.Tuto Dishes Ref` _outactors)
  (bind _foundwidgets (`WidgetBlueprintLibrary.GetAllWidgetsOfClass` "/Game/Blueprints/Widgets/WG_Hud.WG_Hud_C"))
  (set `self.WidgetRef` (`|GetArrayItem` _foundwidgets))
  (bind _returnvalue (`GameplayStatics.SpawnSound2D` "/Game/Audio/Ambient/Menu_01.Menu_01" 1.0 1.0 0.0 null))
  (set `self.ZoukMenu` _returnvalue))

(event `Start Game`
  (for _array_element (`self.Tuto Dishes Ref`)
    (`self.K2_DestroyActor` _array_element))
  (`/Game/Blueprints/Widgets/WG_Hud.DeleteWid` (`self.WidgetRef`)))

(fn `UserConstructionScript`)